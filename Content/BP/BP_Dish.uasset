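; Dish actor that carries dirt patches, which water hits wash away while it tracks cleanliness.
; On BeginPlay it spawns flattened, collision-free cylinder meshes on six axis-aligned faces, each paired with a BP_DirtPatchData object.
; ReceiveWaterHit cleans the first dirty patch matching the local impact normal and current radius, gradually or instantly.
; Patch radius shrinks with the square root of remaining dirt, and cleanliness reaches 100% only when every patch is clean.
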(event EventBeginPlay
  (CallFunction|InitializeDirtPatches))

(event Collision|EventActorBeginOverlap
  (params (OtherActor :type Actor%20Object%20Reference)))

(event EventTick
  (params (DeltaSeconds :type Float%20%28single-precision%29)))

(fn ConstructionScript)

(fn ReceiveWaterHit
  (params (WaterHit :type Hit%20Result%20Structure) (LocalImpactPoint :type Vector) (DeltaSeconds :type Float%20%28double-precision%29))
  (Variables|Default|SetLastWaterHit WaterHit)
  (Variables|Default|SetLastWaterLocalImpact LocalImpactPoint)
  (Variables|Default|SetLastWaterHitDeltaSeconds DeltaSeconds)
  (Variables|Default|SetbWaterHittingActiveDish true)
  (CallFunction|ApplyWaterCleaning LocalImpactPoint (Math|Transform|InverseTransformDirection (Transformation|GetActorTransform) (.ImpactNormal (Collision|BreakHitResult WaterHit))) DeltaSeconds))

(fn ClearWaterHit
  (Variables|Default|SetbWaterHittingActiveDish false)
  (Variables|Default|SetLastWaterHit "")
  (Variables|Default|SetLastWaterLocalImpact "0, 0, 0")
  (Variables|Default|SetLastWaterHitDeltaSeconds 0.0))

(fn InitializeDirtPatches
  (bind _self self)
  (bind _dirtpatchesperface (Variables|Default|GetDirtPatchesPerFace))
  (bind _dirtpatchoffsets (Variables|Default|GetDirtPatchOffsets))
  (bind _dirtpatches (Variables|Default|GetDirtPatches))
  (bind _returnvalue (Utilities|Array|Length _dirtpatchoffsets))
  (bind _returnvalue_2 (Utilities|Array|Length _dirtpatches))
  (bind _returnvalue_3 (Math|Integer|Max(Integer) _dirtpatchesperface))
  (bind _returnvalue_4 (Math|Integer|Min(Integer) _returnvalue_3 _returnvalue))
  (if (== (Utilities|Array|Length (Variables|Default|GetDirtPatches)) (Class|KismetSystemLibrary|MakeLiteralInteger))
    (CallFunction|CreateDirtFace _self 0 "1, 0, 0" _returnvalue_4)
    (CallFunction|CreateDirtFace _self 1 "-1, 0, 0" _returnvalue_4)
    (CallFunction|CreateDirtFace _self 2 "0, 1, 0" _returnvalue_4)
    (CallFunction|CreateDirtFace _self 3 "0, -1, 0" _returnvalue_4)
    (CallFunction|CreateDirtFace _self 4 "0, 0, 1" _returnvalue_4)
    (CallFunction|CreateDirtFace _self 5 "0, 0, -1" _returnvalue_4)
    (Variables|Default|SetTotalDirtPatches _returnvalue_2)
    (Variables|Default|SetRemainingDirtPatches _returnvalue_2)
    (Variables|Default|SetRemainingDirtAmount (Math|Conversions|ToFloat(Integer) _returnvalue_2))
    (Variables|Default|SetbIsFullyClean (== _returnvalue_2 (Class|KismetSystemLibrary|MakeLiteralInteger)))
    (Variables|Default|SetCleanlinessPercent (Math|Float|SelectFloat 1e+02 0.0 (== _returnvalue_2 (Class|KismetSystemLibrary|MakeLiteralInteger))))))

(fn CreateDirtFace
  (params (FaceIndex :type Integer) (Normal :type Vector) (Count :type Integer))
  (for _index (range 0 (- Count (Class|KismetSystemLibrary|MakeLiteralInteger 1)))
    (CallFunction|CreateDirtPatch self FaceIndex _index (+ (* Normal (Math|Float|MakeLiteralFloat 10.12)) (Math|Vector|RotateVector (Utilities|Array|Get(acopy) (Variables|Default|GetDirtPatchOffsets) _index) (Math|Rotator|MakeRotfromZ Normal))) Normal)))

(fn CreateDirtPatch
  (params (FaceIndex :type Integer) (PatchIndex :type Integer) (LocalCenter :type Vector) (LocalNormal :type Vector))
  (bind _self self)
  (bind _returnvalue (Game|ConstructObjectfromClass _self "/Game/BP/BP_DirtPatchData.BP_DirtPatchData_C"))
  (bind _returnvalue_2 (AddComponent|AddStaticMeshComponent _self false (Math|Transform|MakeTransform LocalCenter (Math|Rotator|MakeRotfromZ LocalNormal))))
  (if (and (Utilities|IsValid _returnvalue) (Utilities|IsValid _returnvalue_2))
    (Collision|SetCollisionProfileName _returnvalue_2 "NoCollision" false :!class /Script/Engine.PrimitiveComponent)
    (Components|StaticMesh|SetStaticMesh _returnvalue_2 "/Engine/BasicShapes/Cylinder.Cylinder")
    (Rendering|Material|SetMaterial _returnvalue_2 0 "/Game/BP/M_DirtPatch.M_DirtPatch")
    (Rendering|SetCastShadow _returnvalue_2 false)
    (Variables|/Game/BP/BP_DirtPatchData.BP_DirtPatchData_C|SetPatchId _returnvalue (+ (* FaceIndex (Utilities|Array|Length (Variables|Default|GetDirtPatchOffsets))) PatchIndex))
    (Variables|/Game/BP/BP_DirtPatchData.BP_DirtPatchData_C|SetFaceIndex _returnvalue FaceIndex)
    (Variables|/Game/BP/BP_DirtPatchData.BP_DirtPatchData_C|SetLocalCenter _returnvalue LocalCenter)
    (Variables|/Game/BP/BP_DirtPatchData.BP_DirtPatchData_C|SetLocalNormal _returnvalue LocalNormal)
    (Variables|/Game/BP/BP_DirtPatchData.BP_DirtPatchData_C|SetInitialRadius _returnvalue (Math|Float|Max(Float) 0.01 (Variables|Default|GetDirtPatchRadius)))
    (Variables|/Game/BP/BP_DirtPatchData.BP_DirtPatchData_C|SetDirtAmount _returnvalue 1.0)
    (Variables|/Game/BP/BP_DirtPatchData.BP_DirtPatchData_C|SetVisual _returnvalue _returnvalue_2)
    (CallFunction|UpdateDirtPatchVisual _self _returnvalue)
    (Utilities|Array|Add (Variables|Default|GetDirtPatches) _returnvalue)))

(fn UpdateDirtPatchVisual
  (params (Patch :type BP%20Dirt%20Patch%20Data%20Object%20Reference))
  (bind _returnvalue (Math|Float|MakeLiteralFloat 0.02))
  (bind _visual (Variables|/Game/BP/BP_DirtPatchData.BP_DirtPatchData_C|GetVisual Patch))
  (bind _dirtamount (Variables|/Game/BP/BP_DirtPatchData.BP_DirtPatchData_C|GetDirtAmount Patch))
  (bind _initialradius (Variables|/Game/BP/BP_DirtPatchData.BP_DirtPatchData_C|GetInitialRadius Patch))
  (bind _returnvalue_2 (Math|Float|Sqrt _dirtamount))
  (bind _returnvalue_3 (Math|Float|Max(Float) 0.28 _returnvalue_2))
  (bind _returnvalue_4 (* _initialradius _returnvalue_3))
  (bind _returnvalue_5 (* _returnvalue_4 _returnvalue))
  (Transformation|SetRelativeScale3D _visual (Math|Vector|MakeVector _returnvalue_5 _returnvalue_5 0.001))
  (Rendering|SetVisibility _visual (not (Variables|/Game/BP/BP_DirtPatchData.BP_DirtPatchData_C|GetbIsClean Patch)) false))

(fn SetDirtPatchAmount
  (params (Patch :type BP%20Dirt%20Patch%20Data%20Object%20Reference) (NewAmount :type Float%20%28double-precision%29) (RemovedAmount :type Float%20%28double-precision%29))
  (bind _returnvalue (Math|Float|MakeLiteralFloat 0.0))
  (bind _returnvalue_2 (<= NewAmount _returnvalue))
  (Variables|/Game/BP/BP_DirtPatchData.BP_DirtPatchData_C|SetDirtAmount Patch NewAmount)
  (Variables|/Game/BP/BP_DirtPatchData.BP_DirtPatchData_C|SetbIsClean Patch _returnvalue_2)
  (Variables|Default|SetRemainingDirtPatches (- (Variables|Default|GetRemainingDirtPatches) (Math|Integer|SelectInt 1 0 _returnvalue_2)))
  (Variables|Default|SetRemainingDirtAmount (Math|Float|Max(Float) 0.0 (- (Variables|Default|GetRemainingDirtAmount) RemovedAmount)))
  (Variables|Default|SetbIsFullyClean (== (Variables|Default|GetRemainingDirtPatches) (Class|KismetSystemLibrary|MakeLiteralInteger)))
  (Variables|Default|SetCleanlinessPercent (Math|Float|SelectFloat 1e+02 (Math|Float|Clamp(Float) (* (Math|Float|MakeLiteralFloat 1e+02) (- (Math|Float|MakeLiteralFloat 1.0) (/ (Variables|Default|GetRemainingDirtAmount) (Math|Float|Max(Float) 1.0 (Math|Conversions|ToFloat(Integer) (Variables|Default|GetTotalDirtPatches)))))) 0.0 99.999) (Variables|Default|GetbIsFullyClean)))
  (CallFunction|UpdateDirtPatchVisual self Patch))

(fn ApplyWaterCleaning
  (params (LocalImpactPoint :type Vector) (LocalImpactNormal :type Vector) (DeltaSeconds :type Float%20%28double-precision%29))
  (if (and (not (Variables|Default|GetbIsFullyClean)) (> DeltaSeconds (Math|Float|MakeLiteralFloat 0.0)))
    (bind _array_element (Utilities|Array|ForEachLoopwithBreak (Variables|Default|GetDirtPatches) :!label _label)
      (:LoopBody
        (if (and (not (Variables|/Game/BP/BP_DirtPatchData.BP_DirtPatchData_C|GetbIsClean _array_element)) (> (Math|Vector|DotProduct LocalImpactNormal (Variables|/Game/BP/BP_DirtPatchData.BP_DirtPatchData_C|GetLocalNormal _array_element)) (Math|Float|MakeLiteralFloat 0.99)))
          (if (<= (Math|Vector|VectorLengthSquared (Math|Vector|ProjectVectorontoPlane (- LocalImpactPoint (Variables|/Game/BP/BP_DirtPatchData.BP_DirtPatchData_C|GetLocalCenter _array_element)) (Variables|/Game/BP/BP_DirtPatchData.BP_DirtPatchData_C|GetLocalNormal _array_element))) (* (* (Variables|/Game/BP/BP_DirtPatchData.BP_DirtPatchData_C|GetInitialRadius _array_element) (Math|Float|Max(Float) 0.28 (Math|Float|Sqrt (Variables|/Game/BP/BP_DirtPatchData.BP_DirtPatchData_C|GetDirtAmount _array_element)))) (* (Variables|/Game/BP/BP_DirtPatchData.BP_DirtPatchData_C|GetInitialRadius _array_element) (Math|Float|Max(Float) 0.28 (Math|Float|Sqrt (Variables|/Game/BP/BP_DirtPatchData.BP_DirtPatchData_C|GetDirtAmount _array_element))))))
            (CallFunction|SetDirtPatchAmount self _array_element (Math|Float|SelectFloat 0.0 (Math|Float|Clamp(Float) (- (Variables|/Game/BP/BP_DirtPatchData.BP_DirtPatchData_C|GetDirtAmount _array_element) (/ DeltaSeconds (Math|Float|Max(Float) 0.01 (Variables|Default|GetCleaningTimePerPatch))))) (or (Variables|Default|GetbInstantCleaning) (<= (Math|Float|Clamp(Float) (- (Variables|/Game/BP/BP_DirtPatchData.BP_DirtPatchData_C|GetDirtAmount _array_element) (/ DeltaSeconds (Math|Float|Max(Float) 0.01 (Variables|Default|GetCleaningTimePerPatch))))) (Math|Float|MakeLiteralFloat 1e-05)))) (- (Variables|/Game/BP/BP_DirtPatchData.BP_DirtPatchData_C|GetDirtAmount _array_element) (Math|Float|SelectFloat 0.0 (Math|Float|Clamp(Float) (- (Variables|/Game/BP/BP_DirtPatchData.BP_DirtPatchData_C|GetDirtAmount _array_element) (/ DeltaSeconds (Math|Float|Max(Float) 0.01 (Variables|Default|GetCleaningTimePerPatch))))) (or (Variables|Default|GetbInstantCleaning) (<= (Math|Float|Clamp(Float) (- (Variables|/Game/BP/BP_DirtPatchData.BP_DirtPatchData_C|GetDirtAmount _array_element) (/ DeltaSeconds (Math|Float|Max(Float) 0.01 (Variables|Default|GetCleaningTimePerPatch))))) (Math|Float|MakeLiteralFloat 1e-05))))))
            (goto _label Break)))))))

(fn GetCleanlinessPercent
  (return (Variables|Default|GetCleanlinessPercent)))

(fn IsFullyClean
  (return (Variables|Default|GetbIsFullyClean)))