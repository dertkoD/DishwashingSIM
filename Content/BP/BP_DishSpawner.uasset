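; BP_DishSpawner is an actor that places a single dish in the level when play begins.
; BeginPlay calls SpawnInitialDish, which spawns DishClass at the SpawnPoint component's location and rotation, ignoring collisions.
; It casts the result to BP_Dish, sets its starting DishState and stores it as SpawnedDish, with a DidSpawnDish flag guarding against repeat spawns.
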(event EventBeginPlay
  (CallFunction|SpawnInitialDish))

(event Collision|EventActorBeginOverlap
  (params (OtherActor :type Actor%20Object%20Reference)))

(event EventTick
  (params (DeltaSeconds :type Float%20%28single-precision%29)))

(fn ConstructionScript)

(fn SpawnInitialDish
  (bind _spawnpoint (Variables|Default|GetSpawnPoint))
  (if (not (Variables|Default|GetbDidSpawnDish))
    (bind _returnvalue (Game|SpawnActorfromClass (Variables|Default|GetDishClass) (Math|Transform|MakeTransform (Transformation|GetWorldLocation _spawnpoint) (Transformation|GetWorldRotation _spawnpoint)) "AlwaysSpawn" "MultiplyWithRoot" 0 0))
    (bind _asbp_dish (Utilities|Casting|CastToBP_Dish _returnvalue))
    (Variables|/Game/BP/BP_Dish.BP_Dish_C|SetDishState _asbp_dish "NewEnumerator0")
    (Variables|Default|SetSpawnedDish _asbp_dish)
    (Variables|Default|SetbDidSpawnDish true)))