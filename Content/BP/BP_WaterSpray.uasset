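; Dishwashing water spray actor that the player aims with the mouse at a dish being washed at a sink.
; While spraying, Tick deprojects the cursor, targeting the active dish or a point clamped to a camera-facing plane at the washing anchor.
; A second trace from the sink's water origin stretches the stream mesh, places the impact mesh and applies dish hits.
; Cleanliness gains refresh the owning character's wash prompt.
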(event EventBeginPlay)

(event Collision|EventActorBeginOverlap
  (params (OtherActor :type Actor%20Object%20Reference)))

(event EventTick
  (params (DeltaSeconds :type Float%20%28single-precision%29))
  (CallFunction|UpdateWaterSpray DeltaSeconds))

(fn ConstructionScript)

(fn InitializeWaterSession
  (params (Sink :type BP%20Sink%20Station%20Object%20Reference) (Controller :type Player%20Controller%20Object%20Reference) (PlayerPawn :type Actor%20Object%20Reference))
  (Variables|Default|SetCurrentSink Sink)
  (Variables|Default|SetOwningController Controller)
  (Variables|Default|SetTraceIgnoredActors (Utilities|Array|MakeArray PlayerPawn Sink self (Variables|/Game/BP/BP_SinkStation.BP_SinkStation_C|GetWaterTraceIgnoredHose Sink)))
  (CallFunction|StopWaterSpray))

(fn BeginWaterSpray
  (params (Dish :type BP%20Dish%20Object%20Reference))
  (if (Utilities|IsValid Dish)
    (Variables|Default|SetActiveDish Dish)
    (bind _iscurrent (CallFunction|IsCurrentWaterDish))
    (if _iscurrent
      (Collision|SetActorEnableCollision Dish true)
      (Variables|Default|SetbIsSprayingWater true)
      (Actor|Tick|SetActorTickEnabled self true)
      (else
        (CallFunction|StopWaterSpray)))))

(fn StopWaterSpray
  (Variables|Default|SetbIsSprayingWater false)
  (Actor|Tick|SetActorTickEnabled self)
  (Rendering|SetVisibility (Variables|Default|GetWaterStreamMesh) false false)
  (CallFunction|HideWaterImpact)
  (CallFunction|ClearWaterImpact)
  (if (Utilities|IsValid (Variables|Default|GetActiveDish))
    (Collision|SetActorEnableCollision (Variables|Default|GetActiveDish) false))
  (Variables|Default|SetActiveDish 0)
  (Variables|Default|SetbCameraAimHitsDish false)
  (Variables|Default|SetLastWaterAimTarget "0, 0, 0")
  (Variables|Default|SetLastWaterTraceStart "0, 0, 0")
  (Variables|Default|SetLastWaterTraceEnd "0, 0, 0")
  (Variables|Default|SetLastWaterStreamEnd "0, 0, 0"))

(fn ClearWaterImpact
  (bind _activedish (Variables|Default|GetActiveDish))
  (if (Variables|Default|GetbWaterHittingActiveDish)
    (if (Utilities|IsValid _activedish)
      (Default|ClearWaterHit _activedish))
    (Variables|Default|SetbWaterHittingActiveDish false)))

(fn IsCurrentWaterDish
  (bind _currentsink (Variables|Default|GetCurrentSink))
  (bind _activedish (Variables|Default|GetActiveDish))
  (bind _owningcontroller (Variables|Default|GetOwningController))
  (if (and (Utilities|IsValid _owningcontroller) (and (Utilities|IsValid _currentsink) (Utilities|IsValid _activedish)))
    (if (and (== (Variables|/Game/BP/BP_SinkStation.BP_SinkStation_C|GetActiveDish _currentsink) _activedish) (== (Pawn|GetControlledPawn _owningcontroller) (Components|GetOwner self)))
      (switch Utilities|FlowControl|Switch|SwitchonE_DishState (Variables|/Game/BP/BP_Dish.BP_Dish_C|GetDishState _activedish)
        (:NewEnumerator0
          (return false))
        (:NewEnumerator1
          (return false))
        (:NewEnumerator2
          (return false))
        (:NewEnumerator3
          (return true))
        (:NewEnumerator4
          (return false)))
      (else
        (return false)))
    (else
      (return false))))

(fn ResolveWaterAim
  (bind _returnvalue (Math|Float|MakeLiteralFloat 1.5e+03))
  (bind _owningcontroller (Variables|Default|GetOwningController))
  (bind (_worldlocation _worlddirection _returnvalue_2) (Game|Player|ConvertMouseLocationToWorldSpace _owningcontroller))
  (bind _returnvalue_3 (* _worlddirection _returnvalue))
  (bind _returnvalue_4 (+ _worldlocation _returnvalue_3))
  (Variables|Default|SetbCameraAimHitsDish false)
  (if _returnvalue_2
    (bind (_outhit _returnvalue_5) (Collision|LineTraceByChannel _worldlocation _returnvalue_4 "TraceTypeQuery1" false (Variables|Default|GetTraceIgnoredActors) "None"))
    (if (Variables|Default|GetbDebugWater)
      (Rendering|Debug|DrawDebugLine _worldlocation _returnvalue_4 "(R=0.16,G=0.45,B=1.0,A=1.0)" 0.0 0.3))
    (if (and _returnvalue_5 (== (.HitActor (Collision|BreakHitResult _outhit)) (Variables|Default|GetActiveDish)))
      (Variables|Default|SetbCameraAimHitsDish true)
      (return (.ImpactPoint (Collision|BreakHitResult _outhit)) true)
      (else
        (bind (_target _hastarget) (CallFunction|ClampWaterAimtoWorkspace _worldlocation _returnvalue_4))
        (return _target _hastarget)))
    (else
      (return "0, 0, 0" false))))

(fn ClampWaterAimtoWorkspace
  (params (RayStart :type Vector) (RayEnd :type Vector))
  (bind _returnvalue (Math|Float|MakeLiteralFloat 0.5))
  (bind _returnvalue_2 (Math|Float|MakeLiteralFloat 0.5))
  (bind _currentsink (Variables|Default|GetCurrentSink))
  (bind _wateraimareasize (Variables|Default|GetWaterAimAreaSize))
  (bind (_x _y) (Math|Vector2D|BreakVector2D _wateraimareasize))
  (bind _washinganchor (Variables|/Game/BP/BP_SinkStation.BP_SinkStation_C|GetWashingAnchor _currentsink))
  (bind _washcamera (Variables|/Game/BP/BP_SinkStation.BP_SinkStation_C|GetWashCamera _currentsink))
  (bind _returnvalue_3 (Transformation|GetWorldLocation _washinganchor))
  (bind _returnvalue_4 (Math|Vector|GetForwardVector _washcamera))
  (bind _returnvalue_5 (Math|Vector|GetRightVector _washcamera))
  (bind _returnvalue_6 (Math|Vector|GetUpVector _washcamera))
  (bind _returnvalue_7 (* _x _returnvalue))
  (bind _returnvalue_8 (* _y _returnvalue_2))
  (bind (_t _intersection _returnvalue_9) (Class|KismetMathLibrary|LinePlaneIntersectionOriginNormal RayStart RayEnd _returnvalue_3 _returnvalue_4))
  (bind _returnvalue_10 (- _intersection _returnvalue_3))
  (if _returnvalue_9
    (return (+ _returnvalue_3 (+ (* _returnvalue_5 (Math|Float|Clamp(Float) (Math|Vector|DotProduct _returnvalue_10 _returnvalue_5) (* _returnvalue_7 (Math|Float|MakeLiteralFloat -1.0)) _returnvalue_7)) (* _returnvalue_6 (Math|Float|Clamp(Float) (Math|Vector|DotProduct _returnvalue_10 _returnvalue_6) (* _returnvalue_8 (Math|Float|MakeLiteralFloat -1.0)) _returnvalue_8)))) true)
    (else
      (return "0, 0, 0" false))))

(fn TraceWatertoTarget
  (params (DesiredTarget :type Vector) (DeltaSeconds :type Float%20%28double-precision%29))
  (bind _returnvalue (Math|Float|MakeLiteralFloat 3.0))
  (bind _currentsink (Variables|Default|GetCurrentSink))
  (bind _watermaxdistance (Variables|Default|GetWaterMaxDistance))
  (bind _activedish (Variables|Default|GetActiveDish))
  (bind _waterorigin (Variables|/Game/BP/BP_SinkStation.BP_SinkStation_C|GetWaterOrigin _currentsink))
  (bind _returnvalue_2 (Transformation|GetWorldLocation _waterorigin))
  (bind _returnvalue_3 (- DesiredTarget _returnvalue_2))
  (bind _returnvalue_4 (Math|Vector|VectorLength _returnvalue_3))
  (bind _returnvalue_5 (Math|Vector|Normalize _returnvalue_3))
  (bind _returnvalue_6 (+ _returnvalue_4 _returnvalue))
  (bind _returnvalue_7 (Math|Float|Clamp(Float) _returnvalue_6 0.0 _watermaxdistance))
  (bind _returnvalue_8 (* _returnvalue_5 _returnvalue_7))
  (bind _returnvalue_9 (+ _returnvalue_2 _returnvalue_8))
  (Variables|Default|SetLastWaterAimTarget DesiredTarget)
  (Variables|Default|SetLastWaterTraceStart _returnvalue_2)
  (Variables|Default|SetLastWaterTraceEnd _returnvalue_9)
  (bind (_outhit _returnvalue_10) (Collision|LineTraceByChannel _returnvalue_2 _returnvalue_9 "TraceTypeQuery1" false (Variables|Default|GetTraceIgnoredActors) "None"))
  (if _returnvalue_10
    (CallFunction|RenderWaterSegment _returnvalue_2 (.ImpactPoint (Collision|BreakHitResult _outhit)))
    (CallFunction|ShowWaterImpact (.ImpactPoint (Collision|BreakHitResult _outhit)))
    (if (and (not (.bInitialOverlap (Collision|BreakHitResult _outhit))) (== (.HitActor (Collision|BreakHitResult _outhit)) _activedish))
      (Variables|Default|SetbWaterHittingActiveDish true)
      (CallFunction|ApplyTracedWaterHit _activedish _outhit (Math|Transform|InverseTransformLocation (Transformation|GetActorTransform _activedish) (.ImpactPoint (Collision|BreakHitResult _outhit))) DeltaSeconds)
      (else
        (CallFunction|ClearWaterImpact)))
    (else
      (CallFunction|RenderWaterSegment _returnvalue_2 _returnvalue_9)
      (CallFunction|HideWaterImpact)
      (CallFunction|ClearWaterImpact)))
  (CallFunction|DrawWaterDiagnostics _returnvalue_10))

(fn RenderWaterSegment
  (params (Start :type Vector) (End :type Vector))
  (bind _returnvalue (Math|Float|MakeLiteralFloat 0.02))
  (bind _returnvalue_2 (- End Start))
  (bind _waterstreammesh (Variables|Default|GetWaterStreamMesh))
  (bind _waterstreamradius (Variables|Default|GetWaterStreamRadius))
  (bind _returnvalue_3 (Math|Vector|VectorLength _returnvalue_2))
  (bind _returnvalue_4 (* _waterstreamradius _returnvalue))
  (Variables|Default|SetLastWaterStreamEnd End)
  (if (> _returnvalue_3 (Math|Float|MakeLiteralFloat 0.0001))
    (Transformation|SetWorldLocationAndRotation _waterstreammesh (+ Start (* _returnvalue_2 (Math|Float|MakeLiteralFloat 0.5))) (Math|Rotator|MakeRotfromZ _returnvalue_2) false true)
    (Transformation|SetWorldScale3D _waterstreammesh (Math|Vector|MakeVector _returnvalue_4 _returnvalue_4 (* _returnvalue_3 (Math|Float|MakeLiteralFloat 0.01))))
    (Rendering|SetVisibility _waterstreammesh true false)
    (else
      (Rendering|SetVisibility _waterstreammesh false false))))

(fn DrawWaterDiagnostics
  (params (Blocked :type Boolean))
  (bind _lastwatertracestart (Variables|Default|GetLastWaterTraceStart))
  (bind _lastwaterstreamend (Variables|Default|GetLastWaterStreamEnd))
  (if (Variables|Default|GetbDebugWater)
    (if (Variables|Default|GetbWaterHittingActiveDish)
      (Rendering|Debug|DrawDebugLine _lastwatertracestart _lastwaterstreamend "(R=0.1,G=1.0,B=0.2,A=1.0)" 0.0 1.2)
      (Rendering|Debug|DrawDebugPoint _lastwaterstreamend 7.0 "(R=0.1,G=1.0,B=0.2,A=1.0)" 0.0)
      (else
        (Rendering|Debug|DrawDebugLine _lastwatertracestart _lastwaterstreamend "(R=1.0,G=0.16,B=0.05,A=1.0)" 0.0 1.2)
        (if Blocked
          (Rendering|Debug|DrawDebugPoint _lastwaterstreamend 7.0 "(R=1.0,G=0.16,B=0.05,A=1.0)" 0.0))))))

(fn UpdateWaterSpray
  (params (DeltaSeconds :type Float%20%28double-precision%29))
  (if (Variables|Default|GetbIsSprayingWater)
    (bind _iscurrent (CallFunction|IsCurrentWaterDish))
    (if _iscurrent
      (bind (_target _hastarget) (CallFunction|ResolveWaterAim))
      (if _hastarget
        (CallFunction|TraceWatertoTarget _target DeltaSeconds)
        (else
          (Rendering|SetVisibility (Variables|Default|GetWaterStreamMesh) false false)
          (CallFunction|HideWaterImpact)
          (CallFunction|ClearWaterImpact)))
      (else
        (CallFunction|StopWaterSpray)))))

(fn ShowWaterImpact
  (params (Point :type Vector))
  (bind _waterimpactmesh (Variables|Default|GetWaterImpactMesh))
  (Variables|Default|SetbWaterTraceBlocked true)
  (Transformation|SetWorldLocation _waterimpactmesh Point false true)
  (Transformation|SetWorldScale3D _waterimpactmesh "0.042, 0.042, 0.042")
  (Rendering|SetVisibility _waterimpactmesh true false))

(fn HideWaterImpact
  (Variables|Default|SetbWaterTraceBlocked false)
  (Rendering|SetVisibility (Variables|Default|GetWaterImpactMesh) false false))

(fn ApplyTracedWaterHit
  (params (Dish :type BP%20Dish%20Object%20Reference) (WaterHit :type Hit%20Result%20Structure) (LocalImpactPoint :type Vector) (DeltaSeconds :type Float%20%28double-precision%29))
  (bind _percent (Default|GetCleanlinessPercent Dish))
  (Default|ReceiveWaterHit Dish WaterHit LocalImpactPoint DeltaSeconds)
  (bind _percent_2 (Default|GetCleanlinessPercent Dish))
  (if (> _percent_2 _percent)
    (bind _asbp_first_person_character (Utilities|Casting|CastToBP_FirstPersonCharacter (Components|GetOwner self)))
    (Default|RefreshWashPrompt _asbp_first_person_character)))